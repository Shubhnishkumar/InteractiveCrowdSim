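; Crowd simulation location volume that registers with SimulationManager and collects its child activity points, handing out free ones by requested activity.
; Player overlap with its box shows the location name on the HUD and has NPCManager spawn or despawn its NPCs.
; As a cheap stand-in for distant crowds, linked VisibleLocations show activity-point proxies, capped by simulated student count, while the player is inside, and hide them on exit.
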(event `self.ReceiveBeginPlay`
  (bind _returnvalue (`GameplayStatics.GetActorOfClass` "/Game/interactiveCrowdSIM/NPCManager.NPCManager_C"))
  (set `self.NpcManager` _returnvalue)
  (`self.RegisterActivityPoints`)
  (bind _returnvalue_2 (`GameplayStatics.GetActorOfClass` "/Game/interactiveCrowdSIM/SimulationManager.SimulationManager_C"))
  (set `self.SimulationManager` _returnvalue_2)
  (`/Game/interactiveCrowdSIM/SimulationManager.RegisterLocation` (`self.SimulationManager`) self)
  (bind _asp_character (cast `/Game/Player/P_Character` (`GameplayStatics.GetPlayerPawn` 0)))
  (set `self.Widget` (`/Game/Player/P_Character.widget` _asp_character)))

(event `self.Box.OnComponentBeginOverlap`
  (params (OverlappedComponent :type "PrimitiveComponent Object Reference") (OtherActor :type "Actor Object Reference") (OtherComp :type "PrimitiveComponent Object Reference") (OtherBodyIndex :type Integer) (bFromSweep :type Boolean) (SweepResult :type "HitResult Structure (by ref)"))
  (if (`self.ActorHasTag` OtherActor "Player")
    (`self.PlayerEntered`)
    (bind _widget (`self.Widget`)
      (:`then`
        (`/Game/interactiveCrowdSIM/UIs/playerWidget.ShowLocation` _widget (`KismetTextLibrary.Conv_StringToText` (`KismetSystemLibrary.GetDisplayName` self))))
      (:`else`
        (bind _asp_character (cast `/Game/Player/P_Character` (`GameplayStatics.GetPlayerPawn` 0)))
        (bind _output_get (set `self.Widget` (`/Game/Player/P_Character.widget` _asp_character)))
        (`/Game/interactiveCrowdSIM/UIs/playerWidget.ShowLocation` _output_get (`KismetTextLibrary.Conv_StringToText` (`KismetSystemLibrary.GetDisplayName` self)))))))

(event `/Game/interactiveCrowdSIM/inferface/ICS_Interface.SpawnNPCInteractable`
  (message `/Game/interactiveCrowdSIM/inferface/ICS_Interface.NpcMangerSpawnNPC` (`self.NpcManager`) self (`self.ActivityPointsActor`)))

(event `self.Box.OnComponentEndOverlap`
  (params (OverlappedComponent :type "PrimitiveComponent Object Reference") (OtherActor :type "Actor Object Reference") (OtherComp :type "PrimitiveComponent Object Reference") (OtherBodyIndex :type Integer))
  (if (`self.ActorHasTag` OtherActor "Player")
    (`self.PlayerExited`)
    (`/Game/interactiveCrowdSIM/UIs/playerWidget.ShowLocation` (`self.Widget`) "")))

(fn `AddVisibleStudent`
  (params (StudentCharacter :type "/Game/Player/NPC_Character Object Reference"))
  (bind _visiblestudents (`self.VisiBleStudents`))
  (if (`KismetSystemLibrary.IsValid` StudentCharacter)
    (if (not (`KismetArrayLibrary.Array_Contains` _visiblestudents StudentCharacter))
      (`KismetArrayLibrary.Array_Add` _visiblestudents StudentCharacter))))

(fn `ClearVisibleStudents`
  (`KismetArrayLibrary.Array_Clear` (`self.VisiBleStudents`)))

(fn `FindFreeActivityPoints`
  (params (RequestedActivity :type "/Game/interactiveCrowdSIM/enums/EStudentActivity Enum" :default "NewEnumerator0"))
  (returns (ActivityPoint :type "/Game/interactiveCrowdSIM/Locations/activityPoints/BPActivityPoint Object Reference") (Found :type Boolean))
  (for _array_element (`self.ActivityPointsActor`)
    (if (and (`|EnumEquality` (`/Game/interactiveCrowdSIM/Locations/activityPoints/BPActivityPoint.activity` _array_element) RequestedActivity) (not (`/Game/interactiveCrowdSIM/Locations/activityPoints/BPActivityPoint.IsOccupied` _array_element)))
      (return _array_element true)))
  (return null false))

(fn `GetFreePointForStudent`
  (params (Studentdata :type "/Game/interactiveCrowdSIM/enums/SStudent Structure"))
  (returns (ActivityPoint :type "/Game/interactiveCrowdSIM/Locations/activityPoints/BPActivityPoint Object Reference") (Found :type Boolean))
  (bind (_activitypoint _found) (`self.FindFreeActivityPoints` (`.CurrentActivity_25_99C81EEB4F34933112D04382D6A6227B` (break `/Game/interactiveCrowdSIM/enums/SStudent` Studentdata))))
  (return _activitypoint _found))

(fn `HideActivityPointProxies`
  (for _array_element (`self.ActivityPointsActor`)
    (`/Game/interactiveCrowdSIM/Locations/activityPoints/BPActivityPoint.HideProxy` _array_element)))

(fn `NpcMangerSpawnNPC`
  (params (BpLocation :type "/Game/interactiveCrowdSIM/Locations/BP_Location Object Reference") (array :type "Array of /Game/interactiveCrowdSIM/Locations/activityPoints/BPActivityPoint Object Reference (by ref)"))
  (return))

(fn `PlayerEntered`
  (bind _npcmanager (`self.NpcManager`))
  (bind _locationinfo_locationid (break `/Game/interactiveCrowdSIM/enums/S_Location` (`self.locationinfo`)))
  (set `self.IsPlayerInside` true)
  (`KismetSystemLibrary.PrintString` "entered")
  (if (`KismetSystemLibrary.IsValid` _npcmanager)
    (`KismetSystemLibrary.PrintString` (`KismetStringLibrary.Conv_IntToString` _locationinfo_locationid))
    (`/Game/interactiveCrowdSIM/NPCManager.SpawnLocationNPCs` _npcmanager self)
    (for _array_element (`self.VisibleLocations`)
      (`self.ShowActivityPointProxies` _array_element))))

(fn `PlayerExited`
  (bind _npcmanager (`self.NpcManager`))
  (set `self.IsPlayerInside` false)
  (if (`KismetSystemLibrary.IsValid` _npcmanager)
    (`/Game/interactiveCrowdSIM/NPCManager.DeSpawnLocationNPCs_0` _npcmanager self)
    (`KismetSystemLibrary.PrintString` "exit")
    (for _array_element (`self.VisibleLocations`)
      (`self.HideActivityPointProxies` _array_element))))

(fn `RefreshVisibleStudents`)

(fn `RegisterActivityPoints`
  (`KismetArrayLibrary.Array_Clear` (`self.ActivityPointsActor`))
  (for _array_element (`self.GetAllChildActors` true)
    (bind _asbpactivity_point (cast `/Game/interactiveCrowdSIM/Locations/activityPoints/BPActivityPoint` _array_element))
    (`KismetArrayLibrary.Array_AddUnique` (`self.ActivityPointsActor`) _asbpactivity_point))
  (`KismetSystemLibrary.PrintString` "completed"))

(fn `RemoveVisibleStudent`
  (params (Student :type "/Game/Player/NPC_Character Object Reference"))
  (`KismetArrayLibrary.Array_RemoveItem` (`self.VisiBleStudents`) Student))

(fn `ShowActivityPointProxies`
  (bind _locationinfo_locationid (break `/Game/interactiveCrowdSIM/enums/S_Location` (`self.locationinfo`)))
  (bind _studentsinlocation (`/Game/interactiveCrowdSIM/SimulationManager.GetStudentsInLocation` (`self.SimulationManager`) _locationinfo_locationid))
  (for (_array_element _array_index) (`self.ActivityPointsActor`)
    (if (< _array_index (`KismetArrayLibrary.Array_Length` _studentsinlocation))
      (`/Game/interactiveCrowdSIM/Locations/activityPoints/BPActivityPoint.ShowProxy` _array_element))))

(fn `UserConstructionScript`)